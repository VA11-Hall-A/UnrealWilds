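; BP_Star is a celestial body actor that acts as a gravity source in the game.
; The construction script sets the gravity source's planet radius from the sphere's world X scale.
; On BeginPlay it copies the sphere's mass into the gravity source and registers it with the GravityManager subsystem.
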(event `self.ReceiveBeginPlay`
  (bind _gravitysource (`self.GravitySource`))
  (set `GravitySourceComponent.Mass` (`PrimitiveComponent.GetMass` (`self.Sphere`)) _gravitysource)
  (`GravityManagerSubsystem.RegisterGravitySource` (subsystem `GravityManagerSubsystem`) _gravitysource))

(fn `UserConstructionScript`
  (bind _returnvalue_x (`KismetMathLibrary.BreakVector` (`SceneComponent.K2_GetComponentScale` (`self.Sphere`))))
  (set `GravitySourceComponent.PlanetRadius` _returnvalue_x (`self.GravitySource`)))