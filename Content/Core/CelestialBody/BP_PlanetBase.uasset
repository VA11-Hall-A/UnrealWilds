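; BP_PlanetBase is a base planet Blueprint that derives a starting velocity for a circular orbit around the world origin.
; Its construction script crosses world up with the actor's location for the tangential direction, then scales it by sqrt(GM/r).
; The formula takes a value from OWSettings defaults, uses a hard-coded mass term, and converts between centimeters and meters.
; The result is stored in InitialVelocity; the event graph is empty.
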(fn `UserConstructionScript`
  (bind _returnvalue (`self.K2_GetActorLocation`))
  (set `self.InitialVelocity` (* (* (* (`KismetMathLibrary.Normal` (`KismetMathLibrary.Cross_VectorVector` (0.0 0.0 1.0) _returnvalue) 1e-05) (`KismetMathLibrary.Sqrt` (/ (* (defaults `OWSettings` "/Script/UnrealWilds.OWSettings") 399999991808.0) (/ (`KismetMathLibrary.VSize` _returnvalue) 100.0)))) 100.0) 1.0)))