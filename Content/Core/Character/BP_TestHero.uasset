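; BP_TestHero is a test player hero for a galaxy-scale gravity setup, with mouse or stick look through Enhanced Input.
; On BeginPlay it points its GravityReceiver at Mesh, triggers the GravityManagerSubsystem's galaxy wake-up and adds IMC_Default to the first player.
; Every Tick it moves the world origin to its truncated location, continuously rebasing the world around itself.
; IA_Look feeds controller yaw and pitch; no movement input is handled in this graph.
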(event `self.ReceiveBeginPlay`
  (set `GravityReceiverComponent.TargetPrimitive` (`self.Mesh`) (`self.GravityReceiver`))
  (`GravityManagerSubsystem.TriggerGalaxyWakeUp` (subsystem `GravityManagerSubsystem`))
  (`EnhancedInputSubsystemInterface.AddMappingContext` (pcsubsystem `EnhancedInputLocalPlayerSubsystem` (`GameplayStatics.GetPlayerController` 0)) "/Game/Core/Inputs/IMC_Default.IMC_Default" 0 (struct)))

(event `self.ReceiveTick`
  (params (DeltaSeconds :type "Float (single-precision)"))
  (`GameplayStatics.SetWorldOriginLocation` (`KismetMathLibrary.FTruncVector` (`self.K2_GetActorLocation`))))

(event `EnhancedInput|/Game/Core/Inputs/IA_Look`
  (params (ActionValue :type "Vector2D Structure") (ElapsedSeconds :type "Float (double-precision)") (TriggeredSeconds :type "Float (double-precision)") (InputAction :type "InputAction Object Reference" :default "/Game/Core/Inputs/IA_Look.IA_Look"))
  (:`Triggered`
    (`self.AddControllerYawInput` ActionValue_X)
    (`self.AddControllerPitchInput` ActionValue_Y)))

(fn `UserConstructionScript`)